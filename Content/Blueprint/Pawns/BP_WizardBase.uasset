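; Base wizard pawn that attacks at range by launching power balls at a target actor.
; Attack extends the parent logic: with a valid target and CanAttack set, it spawns BP_WizardPowerBall at the PowerBall component, rotated toward the target.
; The projectile inherits the wizard's IsEnemy flag, and the PowerBall component is hidden after the spawn.
; The construction script only calls the parent, leaving a socket attachment for PowerBall disconnected.
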(event EventBeginPlay
  (|CallParentFunction))

(event EventAttack
  (params (DamagedActor :type Actor%20Object%20Reference))
  (|CallParentFunction DamagedActor)
  (Utilities|IsValid DamagedActor
    (:Is%20Valid
      (if (Variables|Default|GetCanAttack)
        (Game|SpawnActorfromClass "/Game/Blueprint/Actors/BP_WizardPowerBall.BP_WizardPowerBall_C" (Math|Transform|MakeTransform (.location (Transformation|GetWorldTransform (Variables|Default|GetPowerBall))) (Math|Rotator|FindLookatRotation (Transformation|GetWorldLocation (Variables|Default|GetPowerBall)) (Transformation|GetActorLocation DamagedActor)) "1,1,1") "AlwaysSpawn" 0 (Variables|Default|GetIsEnemy) 0)
        (Development|SetHiddeninGame (Variables|Default|GetPowerBall) true false)))))

(fn ConstructionScript
  (|CallParentFunction))