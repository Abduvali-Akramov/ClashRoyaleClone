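; BP_HeroBase is a base combat pawn for heroes on either side, split by an IsEnemy flag, with health and a widget health bar.
; An EnemyVisibility overlap volume tracks opposing heroes in an Enemy array and sets IsEnemyInSphere.
; Attack plays a montage and re-enables CanAttack after a short delay, while AnyDamage updates the bar or destroys the actor.
; Helpers spawn socket-attached weapons and shields; FindEnemy is an empty stub.
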(event OnComponentBeginOverlap(EnemyVisibility)
  (params (OverlappedComponent :type Primitive%20Component%20Object%20Reference) (OtherActor :type Actor%20Object%20Reference) (OtherComp :type Primitive%20Component%20Object%20Reference) (OtherBodyIndex :type Integer) (bFromSweep :type Boolean) (SweepResult :type Hit%20Result%20Structure%20%28by%20ref%29))
  (if (!= OtherActor self)
    (bind _asbp_hero_base (Utilities|Casting|CastToBP_HeroBase OtherActor))
    (if (Math|Boolean|NotEqual(Boolean) (Variables|Default|GetIsEnemy) (Variables|BP_HeroBase_C|GetIsEnemy _asbp_hero_base))
      (Utilities|Array|Add (Variables|Default|GetEnemy) _asbp_hero_base)
      (Variables|Default|SetIsEnemyInSphere true))))

(event OnComponentEndOverlap(EnemyVisibility)
  (params (OverlappedComponent :type Primitive%20Component%20Object%20Reference) (OtherActor :type Actor%20Object%20Reference) (OtherComp :type Primitive%20Component%20Object%20Reference) (OtherBodyIndex :type Integer))
  (bind _asbp_hero_base (Utilities|Casting|CastToBP_HeroBase OtherActor))
  (if (Math|Boolean|NotEqual(Boolean) (Variables|Default|GetIsEnemy) (Variables|BP_HeroBase_C|GetIsEnemy _asbp_hero_base))
    (Utilities|Array|RemoveItem (Variables|Default|GetEnemy) _asbp_hero_base)
    (if (not (!= (Utilities|Array|Length (Variables|Default|GetEnemy)) 0))
      (Variables|Default|SetIsEnemyInSphere false))))

(event Custom|Attack
  (params (DamagedActor :type Actor%20Object%20Reference))
  (Utilities|IsValid DamagedActor
    (:Is%20Valid
      (Utilities|FlowControl|Sequence
        (:then_0
          (Animation|Montage|PlayMontage (Variables|Character|GetMesh) (Variables|Default|GetMontage%20to%20Play)))
        (:then_1
          (Utilities|FlowControl|Delay 0.5)
          (Variables|Default|SetCanAttack true))))))

(event EventBeginPlay
  (bind _aswdb_health_bar (Utilities|Casting|CastToWDB_HealthBar (UserInterface|GetUserWidgetObject (Variables|Default|GetWidget))))
  (Variables|Default|SetAs%20WDB%20Health%20Bar _aswdb_health_bar))

(event Game|Damage|EventAnyDamage
  (params (Damage :type Float%20%28single-precision%29) (DamageType :type Damage%20Type%20Object%20Reference) (InstigatedBy :type Controller%20Object%20Reference) (DamageCauser :type Actor%20Object%20Reference))
  (if (> (- (Variables|Default|GetHealth) Damage) 0.0)
    (bind _output_get (Variables|Default|SetHealth (- (Variables|Default|GetHealth) Damage)))
    (Variables|/Game/UI/Widgets/WDB_HealthBar.WDB_HealthBar_C|SetHealth (Variables|Default|GetAs%20WDB%20Health%20Bar) _output_get)
    (else
      (Actor|DestroyActor))))

(fn ConstructionScript
  (Transformation|SetActorScale3D "2.000000,2.000000,2.000000"))

(fn SpawnWeapon
  (params (InSocketName :type Name) (SocketName :type Name) (Class :type Actor%20Class%20Reference) (Spawn%20Transform%20Scale :type Vector))
  (bind _mesh (Variables|Character|GetMesh))
  (bind _returnvalue (Transformation|GetSocketTransform _mesh InSocketName "RTS_World"))
  (bind _returnvalue_2 (Game|SpawnActorfromClass Class (Math|Transform|MakeTransform (.location _returnvalue) (.rotation _returnvalue) Spawn%20Transform%20Scale) "AlwaysSpawn" 0 0))
  (Transformation|AttachComponentToComponent _returnvalue_2 (Variables|Character|GetMesh) SocketName "SnapToTarget" "SnapToTarget" "SnapToTarget" true))

(fn FindEnemy)

(fn SpawnShield
  (params (Class :type Actor%20Class%20Reference) (InSocketName :type Name) (Spawn%20Transform%20Scale :type Vector) (SocketName :type Name))
  (bind _mesh (Variables|Character|GetMesh))
  (bind _returnvalue (Transformation|GetSocketTransform _mesh InSocketName "RTS_World"))
  (bind _returnvalue_2 (Game|SpawnActorfromClass Class (Math|Transform|MakeTransform (.location _returnvalue) (.rotation _returnvalue) Spawn%20Transform%20Scale) "AlwaysSpawn" 0 0))
  (Transformation|AttachComponentToComponent _returnvalue_2 (Variables|Character|GetMesh) SocketName "SnapToTarget" "SnapToTarget" "SnapToTarget" true))