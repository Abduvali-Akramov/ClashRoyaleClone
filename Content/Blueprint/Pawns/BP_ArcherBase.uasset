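; BP_ArcherBase is an archer pawn Blueprint that extends its parent's attack behavior.
; Its construction script snaps the Weapon component to the BowSocket on the Mesh.
; Attack calls the parent implementation, then applies Damage straight to the target actor if CanAttack is true, with no projectile spawned here.
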(event EventBeginPlay
  (|CallParentFunction))

(event Collision|EventActorBeginOverlap
  (params (OtherActor :type Actor%20Object%20Reference))
  (|CallParentFunction OtherActor) ; This node is disabled and will not be called.\nDrag off pins to build functionality.
)

(event EventTick
  (params (DeltaSeconds :type Float%20%28single-precision%29))
  (|CallParentFunction DeltaSeconds) ; This node is disabled and will not be called.\nDrag off pins to build functionality.
)

(event EventAttack
  (params (DamagedActor :type Actor%20Object%20Reference))
  (|CallParentFunction DamagedActor)
  (if (Variables|Default|GetCanAttack)
    (Game|Damage|ApplyDamage DamagedActor (Variables|Default|GetDamage) 0 0)))

(fn ConstructionScript
  (|CallParentFunction)
  (Transformation|AttachComponentToComponent (Variables|Default|GetWeapon) (Variables|Character|GetMesh) "BowSocket" "SnapToTarget" "SnapToTarget" "SnapToTarget" true))