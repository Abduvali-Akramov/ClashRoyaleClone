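; BP_Castle is a damageable castle actor that tracks its health and displays it on a health bar widget.
; On BeginPlay it caches the WDB_HealthBar from its widget component.
; AnyDamage subtracts damage and pushes the new health to the bar.
; A hit that would bring health to zero or below instead hands the castle to BP_BaseGameMode's DestroyCastle, leaving health and bar unchanged.
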(event EventBeginPlay
  (bind _aswdb_health_bar (Utilities|Casting|CastToWDB_HealthBar (UserInterface|GetUserWidgetObject (Variables|Default|GetWidget))))
  (Variables|Default|SetAs%20WDB%20Health%20Bar _aswdb_health_bar))

(event Game|Damage|EventAnyDamage
  (params (Damage :type Float%20%28single-precision%29) (DamageType :type Damage%20Type%20Object%20Reference) (InstigatedBy :type Controller%20Object%20Reference) (DamageCauser :type Actor%20Object%20Reference))
  (if (> (- (Variables|Default|GetHealth) Damage) 0.0)
    (bind _output_get (Variables|Default|SetHealth (- (Variables|Default|GetHealth) Damage)))
    (Variables|/Game/UI/Widgets/WDB_HealthBar.WDB_HealthBar_C|SetHealth (Variables|Default|GetAs%20WDB%20Health%20Bar) _output_get)
    (else
      (bind _asbp_base_game_mode (Utilities|Casting|CastToBP_BaseGameMode (Game|GetGameMode)))
      (Default|DestroyCastle _asbp_base_game_mode self))))

(fn ConstructionScript)