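; AI controller that acts as an opposing bot player, spawning enemy units on a repeating timer.
; On possession it caches every TargetPoint in the level and starts a looping timer, whose short interval is randomized once at that moment.
; Each tick of the timer spawns a random class from EnemyClasses at a random target point with unit scale, ignoring collisions and setting IsEnemy.
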(event Custom|Spawn%20Enemy%20Event
  (CallFunction|SpawnEnemy (.OutItem (Utilities|Array|Random (Variables|Default|GetEnemy%20Classes))) (.location (Transformation|GetActorTransform (.OutItem (Utilities|Array|Random (stale EventPossess _output_get))))) (.rotation (Transformation|GetActorTransform (.OutItem (Utilities|Array|Random (stale EventPossess _output_get))))) "1.000000,1.000000,1.000000"))

(event EventPossess
  (params (PossessedPawn :type Pawn%20Object%20Reference))
  (bind _outactors (Actor|GetAllActorsOfClass "/Script/Engine.TargetPoint"))
  (bind _output_get (Variables|Default|SetTargets _outactors))
  (Utilities|Time|SetTimerbyEvent (delegate Custom|Spawn%20Enemy%20Event) (Math|Random|RandomFloatinRange 2.0 4.0) true))

(fn ConstructionScript)

(fn SpawnEnemy
  (params (Class :type BP%20Hero%20Base%20Class%20Reference) (Spawn%20Transform%20Location :type Vector) (Spawn%20Transform%20Rotation :type Rotator) (Spawn%20Transform%20Scale :type Vector))
  (Game|SpawnActorfromClass Class (Math|Transform|MakeTransform Spawn%20Transform%20Location Spawn%20Transform%20Rotation Spawn%20Transform%20Scale) "AlwaysSpawn" 0 true 0.0 0))