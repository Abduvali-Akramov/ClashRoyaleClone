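; BP_WizardPowerBall is a wizard power ball actor that deals fixed damage to heroes and castles, then destroys itself.
; Sphere overlap damages a BP_HeroBase only through its capsule and only when the ball's enemy flag differs from the hero's.
; Any overlapped BP_Castle takes the hit without a team check.
; BeginPlay caches the player's hero, which the graph never reads afterward.
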(event OnComponentBeginOverlap(Sphere)
  (params (OverlappedComponent :type Primitive%20Component%20Object%20Reference) (OtherActor :type Actor%20Object%20Reference) (OtherComp :type Primitive%20Component%20Object%20Reference) (OtherBodyIndex :type Integer) (bFromSweep :type Boolean) (SweepResult :type Hit%20Result%20Structure%20%28by%20ref%29))
  (bind _asbp_hero_base (Utilities|Casting|CastToBP_HeroBase OtherActor)
    (:then
      (if (== (Variables|/Script/Engine.Character|GetCapsuleComponent _asbp_hero_base) OtherComp)
        (if (Math|Boolean|NotEqual(Boolean) (Variables|Default|GetIs%20Enemy%20Ball) (Variables|/Game/Blueprint/Pawns/BP_HeroBase.BP_HeroBase_C|GetIsEnemy _asbp_hero_base))
          (Game|Damage|ApplyDamage OtherActor 1e+01 0 0 :!label _label)
          (Actor|DestroyActor))))
    (:CastFailed
      (Utilities|Casting|CastToBP_Castle OtherActor)
      (goto _label))))

(event EventBeginPlay
  (bind _asbp_hero_base (Utilities|Casting|CastToBP_HeroBase (Game|Player|GetPlayerPawn 0)))
  (Variables|Default|SetAs%20BP%20Hero%20Base _asbp_hero_base))

(fn ConstructionScript)