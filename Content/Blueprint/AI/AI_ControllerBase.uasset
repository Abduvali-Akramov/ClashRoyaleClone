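; Base AI controller that drives a BP_HeroBase unit to attack nearby enemies or opposing castles.
; On possess it caches the hero's team and attack radius, then re-evaluates targets on a looping timer.
; It moves to the nearest enemy detected in the hero's sphere, or otherwise the nearest opposing castle, and calls Attack on arrival.
; The controller destroys itself on unpossess.
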(event Custom|Find%20Enemy%20and%20Follow
  (bind _returnvalue (Pawn|GetControlledPawn))
  (if (Variables|/Game/Blueprint/Pawns/BP_HeroBase.BP_HeroBase_C|GetIsEnemyInSphere (Variables|Default|GetHero%20Ref))
    (bind _output_get (Variables|Default|SetClosest%20target (Utilities|Array|Get(acopy) (Variables|/Game/Blueprint/Pawns/BP_HeroBase.BP_HeroBase_C|GetEnemy (Variables|Default|GetHero%20Ref)))))
    (Utilities|IsValid _output_get
      (:Is%20Valid
        (for _array_element (Variables|/Game/Blueprint/Pawns/BP_HeroBase.BP_HeroBase_C|GetEnemy (Variables|Default|GetHero%20Ref))
          (Utilities|IsValid _array_element
            (:Is%20Valid
              (if (<= (Transformation|GetDistanceTo _array_element _returnvalue) (Transformation|GetDistanceTo (Variables|Default|GetClosest%20target) _returnvalue))
                (Variables|Default|SetClosest%20target _array_element)))))
        (AI|AIMoveTo (Pawn|GetControlledPawn) "0, 0, 0" (Variables|Default|GetClosest%20target) (Variables|Default|GetMy%20Radius) false
          (:OnSuccess
            (Default|Attack (Variables|Default|GetHero%20Ref) (Variables|Default|GetClosest%20target))))))
    (else
      (CallFunction|FollowCastle))))

(event Custom|Follow%20Castle
  (bind _returnvalue (Pawn|GetControlledPawn))
  (bind _castles (Variables|Default|GetCastles))
  (bind _output (Utilities|Array|Get(acopy) _castles))
  (Utilities|Array|Clear (Variables|Default|GetCastles))
  (bind _outactors (Actor|GetAllActorsOfClass "/Game/Blueprint/Actors/BP_Castle.BP_Castle_C"))
  (for _array_element _outactors
    (if (Math|Boolean|NotEqual(Boolean) (Variables|Default|GetMy%20enemy) (Variables|/Game/Blueprint/Actors/BP_Castle.BP_Castle_C|GetIsEnemyCastle _array_element))
      (Utilities|Array|Add (Variables|Default|GetCastles) _array_element)))
  (Utilities|IsValid _output
    (:Is%20Valid
      (Variables|Default|SetClosest%20Castle _output)
      (for _array_element_2 (Variables|Default|GetCastles)
        (Utilities|IsValid _array_element_2
          (:Is%20Valid
            (if (<= (Transformation|GetDistanceTo _array_element_2 _returnvalue) (Transformation|GetDistanceTo (Variables|Default|GetClosest%20Castle) _returnvalue))
              (Variables|Default|SetClosest%20Castle _array_element_2)))))
      (AI|AIMoveTo (Pawn|GetControlledPawn) "0, 0, 0" (Variables|Default|GetClosest%20Castle) 5e+02 false
        (:OnSuccess
          (Default|Attack (Variables|Default|GetHero%20Ref) (Variables|Default|GetClosest%20Castle)))))))

(event EventUnPossess
  (params (UnpossessedPawn :type Pawn%20Object%20Reference))
  (Actor|DestroyActor))

(event EventPossess
  (params (PossessedPawn :type Pawn%20Object%20Reference))
  (Utilities|FlowControl|Sequence
    (:then_0
      (bind _asbp_hero_base (Utilities|Casting|CastToBP_HeroBase PossessedPawn))
      (Variables|Default|SetHero%20Ref _asbp_hero_base)
      (Variables|Default|SetMy%20enemy (Variables|/Game/Blueprint/Pawns/BP_HeroBase.BP_HeroBase_C|GetIsEnemy _asbp_hero_base))
      (CallFunction|FindEnemyandFollow)
      (Utilities|Time|SetTimerbyEvent (delegate Custom|Find%20Enemy%20and%20Follow) (Variables|Default|GetTime) true))
    (:then_1
      (Variables|Default|SetMy%20Radius (Variables|/Game/Blueprint/Pawns/BP_HeroBase.BP_HeroBase_C|GetRadius (Variables|Default|GetHero%20Ref))))))

(event EventBeginPlay)

(fn ConstructionScript)