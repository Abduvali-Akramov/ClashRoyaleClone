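; Base game mode for a castle-versus-castle match, deciding when it ends and who wins.
; BeginPlay shows the mouse cursor and starts a match timer.
; Destroying a castle increments the score and runs EndTimer, the same function the timer calls.
; EndTimer counts castles per side and, when either side has none or time runs out, pauses and shows a win, draw or lose widget.
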(event Custom|Destroy%20Castle
  (params (Destroyed%20Actor :type Actor%20Object%20Reference))
  (Actor|DestroyActor Destroyed%20Actor)
  (Math|Integer|IncrementInt (Variables|Default|GetScore)
    (:%20%20
      (CallFunction|EndTimer))))

(event EventBeginPlay
  (Utilities|FlowControl|Sequence
    (:then_0
      (Variables|/Script/Engine.PlayerController|SetbShowMouseCursor (Game|GetPlayerController 0) true))
    (:then_1
      (bind _returnvalue (Utilities|Time|SetTimerbyFunctionName self "EndTimer" (Variables|Default|GetTime)))
      (Variables|Default|SetTimer _returnvalue))))

(fn ConstructionScript)

(fn EndTimer
  (Variables|Default|SetEnemy 0)
  (Variables|Default|SetPlayer 0)
  (bind _outactors (Actor|GetAllActorsOfClass "/Game/Blueprint/Actors/BP_Castle.BP_Castle_C"))
  (for _array_element _outactors
    (if (Variables|/Game/Blueprint/Actors/BP_Castle.BP_Castle_C|GetIsEnemyCastle _array_element)
      (Math|Integer|IncrementInt (Variables|Default|GetEnemy))
      (else
        (Math|Integer|IncrementInt (Variables|Default|GetPlayer)))))
  (if (or (== (Variables|Default|GetEnemy) 0) (== (Variables|Default|GetPlayer) 0))
    (bind _returnvalue (UserInterface|CreateWidget "/Game/UI/Widgets/WDB_WinLose.WDB_WinLose_C" :!label _label))
    (UserInterface|Viewport|AddtoViewport _returnvalue 0)
    (Game|SetGamePaused true)
    (Math|Integer|CompareInt (Variables|Default|GetPlayer) (Variables|Default|GetEnemy)
      (:>
        (Rendering|Components|TextRender|SetText (Variables|/Game/UI/Widgets/WDB_WinLose.WDB_WinLose_C|GetText _returnvalue) "Win!"))
      (:==
        (Rendering|Components|TextRender|SetText (Variables|/Game/UI/Widgets/WDB_WinLose.WDB_WinLose_C|GetText _returnvalue) "DRAW!"))
      (:<
        (Rendering|Components|TextRender|SetText (Variables|/Game/UI/Widgets/WDB_WinLose.WDB_WinLose_C|GetText _returnvalue) "Oh shit! You lose!")))
    (elif (not (>= (Utilities|Time|GetTimerRemainingTimebyHandle (Variables|Default|GetTimer)) 0.1))
      (goto _label))))